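; BP_light is a light-puzzle trigger in level 3 that opens a door when a light gap wall sits above it.
; It caches its Cube's world location at BeginPlay as the trace origin.
; While the referenced Light's flag is on, Tick line-traces straight up on the Visibility channel.
; Every tick the trace hits a BP_lightGapWall, it calls Open on the referenced Door, with no close or one-shot guard.
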(event `self.ReceiveBeginPlay`
  (set `self.start loc` (`SceneComponent.K2_GetComponentLocation` (`self.Cube`))))

(event `self.ReceiveTick`
  (params (DeltaSeconds :type "Float (single-precision)"))
  (bind _start_loc (`self.start loc`))
  (if (`/Game/2D3D/level3/BP_LightArea.light?` (`self.light`))
    (bind _outhit (`KismetSystemLibrary.LineTraceSingle` _start_loc (`KismetMathLibrary.MakeVector` (.x _start_loc) (.y _start_loc) (+ (.z _start_loc) 1000.0)) "TraceTypeQuery1"))
    (cast `/Game/2D3D/level3/BP_lightGapWall` (`.HitActor` (`GameplayStatics.BreakHitResult` _outhit)))
    (`/Game/2D3D/level3/BP_Door.open` (`self.door`))))

(fn `UserConstructionScript`)