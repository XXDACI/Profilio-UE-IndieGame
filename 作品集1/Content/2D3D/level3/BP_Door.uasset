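; BP_Door is a double sliding door in level3 that opens once until reset.
; Open sets a lock and runs two timelines that slide the leaves apart along world Y from positions cached at BeginPlay.
; Reset snaps both leaves back and clears the lock without rewinding the timelines.
; The left timeline uses PlayFromStart but the right uses Play, so only the left restarts on a later open.
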(event `self.ReceiveBeginPlay`
  (set `self.leftStartloc` (`SceneComponent.K2_GetComponentLocation` (`self.door left`)))
  (set `self.rightStartloc` (`SceneComponent.K2_GetComponentLocation` (`self.door right`))))

(event `open`
  (if (not (`self.lock`))
    (`self.left open`)
    (`self.right open`)
    (set `self.lock` true)))

(event `left open`
  (bind (_direction _newtrack_0) (`Timeline|Timeline` :!via `PlayFromStart`)
    (:`Update`
      (`SceneComponent.K2_SetWorldLocation` (`self.door left`) (`KismetMathLibrary.MakeVector` (.x (`self.leftStartloc`)) (- (.y (`self.leftStartloc`)) (* _newtrack_0 250.0)) (.z (`self.leftStartloc`))) false false))))

(event `right open`
  (bind (_direction _newtrack_0) (`Timeline|Timeline_0`)
    (:`Update`
      (`SceneComponent.K2_SetWorldLocation` (`self.door right`) (`KismetMathLibrary.MakeVector` (.x (`self.rightStartloc`)) (+ (* _newtrack_0 250.0) (.y (`self.rightStartloc`))) (.z (`self.rightStartloc`))) false false))))

(event `reset`
  (`SceneComponent.K2_SetWorldLocation` (`self.door left`) (`self.leftStartloc`) false false)
  (`SceneComponent.K2_SetWorldLocation` (`self.door right`) (`self.rightStartloc`) false false)
  (set `self.lock` false))

(fn `UserConstructionScript`)