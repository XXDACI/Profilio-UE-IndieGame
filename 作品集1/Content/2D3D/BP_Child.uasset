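; BP_Child is a child Blueprint in the 2D3D folder that reshapes the collision box it uses when play begins.
; BeginPlay runs the parent logic, then calls ChangeSelfColl.
; Its ChangeSelfColl override stretches the Box component far along the Y axis and updates overlaps, without running the parent version.
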(event `self.ReceiveBeginPlay`
  (`parent.ReceiveBeginPlay`)
  (`self.ChangeSelfColl`))

(fn `ChangeSelfColl`
  (`BoxComponent.SetBoxExtent` (`self.Box`) (50.0 1000.0 50.0) true))

(fn `UserConstructionScript`
  (`parent.UserConstructionScript`))