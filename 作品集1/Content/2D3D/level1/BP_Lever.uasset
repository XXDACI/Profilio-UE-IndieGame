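; BP_Lever is a level lever that spawns a BP_Lava actor when pulled.
; pullLever clears the LeverLock gate, then a timeline lerps the Lever component's rotation and position to the thrown pose.
; On finish it spawns the lava at the referenced Box actor's location and calls the reset, whose second timeline swings the lever back and re-arms the gate.
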(event `pullLever`
  (bind _lever (`self.lever`))
  (if (`self.leverLock`)
    (set `self.leverLock` false)
    (bind (_direction _alpha) (`Timeline|Timeline` :!via `PlayFromStart`)
      (:`Update`
        (`SceneComponent.K2_SetRelativeRotation` _lever (`KismetMathLibrary.RLerp` (struct :`Pitch` 30.0) (struct :`Pitch` -30.0) _alpha) false false)
        (`SceneComponent.K2_SetRelativeLocation` _lever (`KismetMathLibrary.VLerp` (-6.062178 0.0 16.5) (6.062178 0.0 16.5) _alpha) false false))
      (:`Finished`
        (`|SpawnActorFromClass` "/Game/2D3D/level1/trape/BP_Lava.BP_Lava_C" (`KismetMathLibrary.MakeTransform` (`self.K2_GetActorLocation` (`self.box`))) "Undefined" "MultiplyWithRoot" null 0.0 null)
        (`self.resetLever`)))))

(event `resetLever`
  (bind _lever (`self.lever`))
  (bind (_direction _alpha) (`Timeline|Timeline_0` :!via `PlayFromStart`)
    (:`Update`
      (`SceneComponent.K2_SetRelativeRotation` _lever (`KismetMathLibrary.RLerp` (struct :`Pitch` -30.0) (struct :`Pitch` 30.0) _alpha) false false)
      (`SceneComponent.K2_SetRelativeLocation` _lever (`KismetMathLibrary.VLerp` (6.062178 0.0 16.5) (-6.062178 0.0 16.5) _alpha) false false))
    (:`Finished`
      (set `self.leverLock` true))))

(fn `UserConstructionScript`)