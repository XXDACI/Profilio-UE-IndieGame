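; BP_Bridges is a level 1 Blueprint with Left and Right bridge components, only one of which keeps collision each play.
; On BeginPlay, RandomizeBridge makes a coin-flip choice between the two sides.
; The chosen side loses collision and gets MI_Cube_03, while the other gets query-only collision and BasicShapeMaterial.
; A debug print names the side that lost collision.
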(event `self.ReceiveBeginPlay`
  (`self.RandomizeBridge`))

(fn `RandomizeBridge`
  (bind _right (`self.right`))
  (bind _left (`self.left`))
  (bind _right_2 (`self.right`))
  (bind _left_2 (`self.left`))
  (if (== (`KismetMathLibrary.RandomInteger` 2) 1)
    (`PrimitiveComponent.SetCollisionEnabled` _left_2 "NoCollision")
    (`PrimitiveComponent.SetMaterial` _left_2 0 "/Engine/VREditor/BasicMeshes/MI_Cube_03.MI_Cube_03")
    (`PrimitiveComponent.SetCollisionEnabled` _right "QueryOnly")
    (`PrimitiveComponent.SetMaterial` _right 0 "/Engine/BasicShapes/BasicShapeMaterial.BasicShapeMaterial")
    (`KismetSystemLibrary.PrintString` "left" true true (struct :`G` 0.66 :`B` 1.0 :`A` 1.0) 100.0)
    (else
      (`PrimitiveComponent.SetCollisionEnabled` _right_2 "NoCollision")
      (`PrimitiveComponent.SetMaterial` _right_2 0 "/Engine/VREditor/BasicMeshes/MI_Cube_03.MI_Cube_03")
      (`PrimitiveComponent.SetCollisionEnabled` _left "QueryOnly")
      (`PrimitiveComponent.SetMaterial` _left 0 "/Engine/BasicShapes/BasicShapeMaterial.BasicShapeMaterial")
      (`KismetSystemLibrary.PrintString` "right" true true (struct :`G` 0.66 :`B` 1.0 :`A` 1.0) 100.0))))

(fn `UserConstructionScript`)