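; Elevator trap-folder actor that lifts two boxes, BoxB and BoxC, while something overlaps its Box trigger and lowers them when the overlap ends.
; Start locations are cached on BeginPlay, and each box has its own timeline that plays on rise and reverses on descent.
; Timeline values scale a Z offset from the origin, lifting BoxC roughly twice as high as BoxB via teleporting location updates.
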(event `self.ReceiveBeginPlay`
  (set `self.bOrigin` (`self.K2_GetActorLocation` (`self.boxB`)))
  (set `self.cOrigin` (`self.K2_GetActorLocation` (`self.boxC`))))

(event `self.Box.OnComponentBeginOverlap`
  (params (OverlappedComponent :type "PrimitiveComponent Object Reference") (OtherActor :type "Actor Object Reference") (OtherComp :type "PrimitiveComponent Object Reference") (OtherBodyIndex :type Integer) (bFromSweep :type Boolean) (SweepResult :type "HitResult Structure (by ref)"))
  (`self.b_rise`)
  (`self.c_rise`))

(event `self.Box.OnComponentEndOverlap`
  (params (OverlappedComponent :type "PrimitiveComponent Object Reference") (OtherActor :type "Actor Object Reference") (OtherComp :type "PrimitiveComponent Object Reference") (OtherBodyIndex :type Integer))
  (`self.b_down`)
  (`self.c_down`))

(event `b_rise`
  (bind (_direction _tl_lift) (`Timeline|Timeline` :`NewTime` (`self.btime`) :!label _label)
    (:`Update`
      (set `self.btime` _tl_lift)
      (`self.K2_SetActorLocation` (`self.boxB`) (`KismetMathLibrary.MakeVector` (.x (`self.bOrigin`)) (.y (`self.bOrigin`)) (+ (* _tl_lift 105.0) (.z (`self.bOrigin`)))) false true))))

(event `b_down`
  (goto _label :!via `Reverse`))

(event `c_rise`
  (bind (_direction _tl_lift) (`Timeline|Timeline_0` :`NewTime` (`self.ctime`) :!label _label_2)
    (:`Update`
      (set `self.ctime` _tl_lift)
      (`self.K2_SetActorLocation` (`self.boxC`) (`KismetMathLibrary.MakeVector` (.x (`self.cOrigin`)) (.y (`self.cOrigin`)) (+ (* _tl_lift 215.0) (.z (`self.cOrigin`)))) false true))))

(event `c_down`
  (goto _label_2 :!via `Reverse`))

(fn `UserConstructionScript`
  (`parent.UserConstructionScript`))