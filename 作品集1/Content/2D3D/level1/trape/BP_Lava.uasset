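; BP_Lava is a short-lived lava hazard that deals heavy damage to the third-person character on contact.
; Every tick it reads the player's 2D flag and switches its box collision extent between NewSize and OldSize to suit the current perspective.
; Overlapping that box calls Hurt on the character, and a Tick-accumulated timer destroys the actor after about five seconds.
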(event `self.ReceiveBeginPlay`)

(event `self.ReceiveTick`
  (params (DeltaSeconds :type "Float (single-precision)"))
  (bind _box (`self.Box`))
  (bind _asbp_third_person_character (cast `/Game/ThirdPerson/Blueprints/BP_ThirdPersonCharacter` (`GameplayStatics.GetPlayerCharacter` 0)))
  (if (`/Game/ThirdPerson/Blueprints/BP_ThirdPersonCharacter.2D?` _asbp_third_person_character)
    (`BoxComponent.SetBoxExtent` _box (`self.new size`) true)
    (else
      (`BoxComponent.SetBoxExtent` _box (`self.old size`) true)))
  (bind _output_get (set `self.time` (+ DeltaSeconds (`self.time`))))
  (if (> _output_get 5.0)
    (`self.K2_DestroyActor`)))

(event `self.Box.OnComponentBeginOverlap`
  (params (OverlappedComponent :type "PrimitiveComponent Object Reference") (OtherActor :type "Actor Object Reference") (OtherComp :type "PrimitiveComponent Object Reference") (OtherBodyIndex :type Integer) (bFromSweep :type Boolean) (SweepResult :type "HitResult Structure (by ref)"))
  (bind _asbp_third_person_character (cast `/Game/ThirdPerson/Blueprints/BP_ThirdPersonCharacter` OtherActor))
  (`/Game/ThirdPerson/Blueprints/BP_ThirdPersonCharacter.Hurt` _asbp_third_person_character 100.0))

(fn `UserConstructionScript`
  (`parent.UserConstructionScript`))