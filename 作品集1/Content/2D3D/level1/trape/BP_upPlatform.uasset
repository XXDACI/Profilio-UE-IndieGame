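; Platform actor for the 2D/3D level that pushes the player character upward on contact.
; Each Tick reads the player's 2D flag and stretches the cube along Y while in 2D, restoring uniform scale otherwise.
; Overlapping its box instantly moves the character up by a fixed offset without sweeping, stops the player's movement and calls 3DLock on the character.
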(event `self.ReceiveTick`
  (params (DeltaSeconds :type "Float (single-precision)"))
  (bind _cube (`self.Cube`))
  (bind _asbp_third_person_character (cast `/Game/ThirdPerson/Blueprints/BP_ThirdPersonCharacter` (`GameplayStatics.GetPlayerCharacter` 0)))
  (if (`/Game/ThirdPerson/Blueprints/BP_ThirdPersonCharacter.2D?` _asbp_third_person_character)
    (`SceneComponent.SetRelativeScale3D` _cube (1.0 20.0 1.0))
    (else
      (`SceneComponent.SetRelativeScale3D` _cube (1.0 1.0 1.0)))))

(event `self.Box.OnComponentBeginOverlap`
  (params (OverlappedComponent :type "PrimitiveComponent Object Reference") (OtherActor :type "Actor Object Reference") (OtherComp :type "PrimitiveComponent Object Reference") (OtherBodyIndex :type Integer) (bFromSweep :type Boolean) (SweepResult :type "HitResult Structure (by ref)"))
  (bind _asbp_third_person_character (cast `/Game/ThirdPerson/Blueprints/BP_ThirdPersonCharacter` OtherActor))
  (`self.K2_SetActorLocation` _asbp_third_person_character (`KismetMathLibrary.MakeVector` (.x (`self.K2_GetActorLocation` _asbp_third_person_character)) (.y (`self.K2_GetActorLocation` _asbp_third_person_character)) (+ (.z (`self.K2_GetActorLocation` _asbp_third_person_character)) 200.0)) false false)
  (`MovementComponent.StopMovementImmediately` (`Character.CharacterMovement` (`GameplayStatics.GetPlayerCharacter` 0)))
  (`/Game/ThirdPerson/Blueprints/BP_ThirdPersonCharacter.3DLock` _asbp_third_person_character))

(fn `UserConstructionScript`
  (`parent.UserConstructionScript`))