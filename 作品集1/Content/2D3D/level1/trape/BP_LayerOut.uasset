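; BP_LayerOut is a trigger actor in level 1 that opens up the layer 2 door when a key box enters it.
; On BeginPlay it finds BP_DoorToLayer2 actors tagged "layer2Door" and keeps the last one found.
; When a BP_BoxKey overlaps its Box component, it prints a debug string, sets that door's Out flag and calls Appear on it.
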(event `self.ReceiveBeginPlay`
  (bind _outactors (`GameplayStatics.GetAllActorsOfClassWithTag` "/Game/2D3D/level2/level2_destinyfeature/BP_DoorToLayer2.BP_DoorToLayer2_C" "layer2Door"))
  (for _array_element _outactors
    (set `self.doorLayer2` _array_element)))

(event `self.Box.OnComponentBeginOverlap`
  (params (OverlappedComponent :type "PrimitiveComponent Object Reference") (OtherActor :type "Actor Object Reference") (OtherComp :type "PrimitiveComponent Object Reference") (OtherBodyIndex :type Integer) (bFromSweep :type Boolean) (SweepResult :type "HitResult Structure (by ref)"))
  (cast `/Game/2D3D/level1/BP_BoxKey` OtherActor)
  (`KismetSystemLibrary.PrintString` "real")
  (bind _asbp_door_to_layer_2 (cast `/Game/2D3D/level2/level2_destinyfeature/BP_DoorToLayer2` (`self.doorLayer2`)))
  (set `/Game/2D3D/level2/level2_destinyfeature/BP_DoorToLayer2.out?` true _asbp_door_to_layer_2)
  (`/Game/2D3D/level2/level2_destinyfeature/BP_DoorToLayer2.appear` _asbp_door_to_layer_2))

(fn `UserConstructionScript`
  (`parent.UserConstructionScript`))