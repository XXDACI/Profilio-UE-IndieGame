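; BP_Tablet is a trigger that teleports the third-person character to one of two layer locations and sets up that layer's challenge.
; Its box overlap picks the destination from the Layer2 flag, which the reset event clears.
; Layer 1 spawns a next-layer key in one of six random slots, then starts the rolling rock after a delay.
; Layer 2 respawns BoxKey, randomizes KeyTablet's platform and hides LayerOut.
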(event `self.ReceiveTick`
  (params (DeltaSeconds :type "Float (single-precision)")))

(event `self.Box.OnComponentBeginOverlap`
  (params (OverlappedComponent :type "PrimitiveComponent Object Reference") (OtherActor :type "Actor Object Reference") (OtherComp :type "PrimitiveComponent Object Reference") (OtherBodyIndex :type Integer) (bFromSweep :type Boolean) (SweepResult :type "HitResult Structure (by ref)"))
  (bind _asbp_third_person_character (cast `/Game/ThirdPerson/Blueprints/BP_ThirdPersonCharacter` OtherActor))
  (if (`self.layer2`)
    (`self.K2_SetActorLocation` _asbp_third_person_character (`self.layer2cor`) false false)
    (`self.layer 2 stuff`)
    (else
      (`self.K2_SetActorLocation` _asbp_third_person_character (`self.layer1cor`) false false)
      (`self.layer1Stuff`))))

(event `layer1Stuff`
  (bind _rollingrockref (`self.RollingRockRef`))
  (`|SpawnActorFromClass` "/Game/2D3D/level2/level2_destinyfeature/BP_KeyToNextLayer.BP_KeyToNextLayer_C" (`KismetMathLibrary.MakeTransform` (`KismetMathLibrary.Conv_IntVectorToVector` (make `IntVector` (+ (* (`KismetMathLibrary.RandomInteger` 6) 1200) 384) 1000 -40020))) "Undefined" "MultiplyWithRoot" null null)
  (`KismetSystemLibrary.PrintString` "spawn")
  (`KismetSystemLibrary.Delay` 5.0)
  (`KismetSystemLibrary.PrintString` (`KismetSystemLibrary.GetDisplayName` _rollingrockref))
  (`/Game/2D3D/level2/level2_destinyfeature/BP_RollingRock.StartRoll` _rollingrockref))

(event `layer 2 stuff`
  (`/Game/2D3D/level1/BP_BoxKey.respawn` (`self.BoxKey`))
  (`/Game/2D3D/level2/level2_destinyfeature/BP_KeyTablet.randomPlatform` (`self.KeyTablet`))
  (`/Game/2D3D/level2/level2_destinyfeature/BP_DoorToLayer2.hide` (`self.layerOut`)))

(event `reset`
  (set `self.layer2` false))

(fn `UserConstructionScript`
  (`parent.UserConstructionScript`))