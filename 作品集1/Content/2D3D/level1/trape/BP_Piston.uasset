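; Piston trap that slides its Cube endlessly back and forth along world Y, up to 2000 units from its starting location.
; BeginPlay stores that start location, then the Dirction variable picks whether the cycle opens with the forward or back stroke.
; Two timelines drive the position without sweep and restart each other on finish, so the back start begins at the far end.
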(event `self.ReceiveBeginPlay`
  (set `self.startloc` (`SceneComponent.K2_GetComponentLocation` (`self.Cube`)))
  (if (== (`self.dirction`) 0)
    (`self.forward`)
    (else
      (`self.back`))))

(event `self.ReceiveTick`
  (params (DeltaSeconds :type "Float (single-precision)")))

(event `forward`
  (bind (_direction _alpha) (`Timeline|Timeline` :`NewTime` 0.5 :!via `PlayFromStart` :!label _label)
    (:`Update`
      (`SceneComponent.K2_SetWorldLocation` (`self.Cube`) (`KismetMathLibrary.MakeVector` (.x (`self.startloc`)) (+ (* _alpha 2000.0) (.y (`self.startloc`))) (.z (`self.startloc`))) false false))
    (:`Finished`
      (bind (_direction_2 _alpha_2) (`Timeline|Timeline_0` :`NewTime` 0.5 :!via `ReverseFromEnd` :!label _label_2)
        (:`Update`
          (`SceneComponent.K2_SetWorldLocation` (`self.Cube`) (`KismetMathLibrary.MakeVector` (.x (`self.startloc`)) (+ (* _alpha_2 2000.0) (.y (`self.startloc`))) (.z (`self.startloc`))) false false))
        (:`Finished`
          (goto _label :!via `PlayFromStart`))))))

(event `back`
  (goto _label_2 :!via `ReverseFromEnd`))

(fn `UserConstructionScript`
  (`parent.UserConstructionScript`))