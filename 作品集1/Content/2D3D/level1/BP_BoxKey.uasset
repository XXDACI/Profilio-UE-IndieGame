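; BP_BoxKey is a physics cube, named as a key box, that returns to its start when it falls for too long.
; BeginPlay stores the starting transform, and Tick traces 200 units downward with per-frame debug drawing to check for ground.
; Time without a hit accumulates until it exceeds MaxFallingTime, triggering a respawn.
; Respawn restores the stored transform, zeroes the cube's linear and angular velocity, and resets the timer.
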(event `self.ReceiveBeginPlay`
  (set `self.StartTransform` (`self.GetTransform`))
  (set `self.originLoc` (`self.K2_GetActorLocation`)))

(event `self.ReceiveTick`
  (params (DeltaSeconds :type "Float (single-precision)"))
  (bind (_outhits _returnvalue) (`KismetSystemLibrary.LineTraceMulti` :`Start` (`self.K2_GetActorLocation`) :`End` (+ (`self.K2_GetActorLocation`) (0.0 0.0 -200.0)) :`TraceChannel` "TraceTypeQuery1" :`DrawDebugType` "ForOneFrame"))
  (if _returnvalue
    (set `self.FallingTime` 0.0)
    (else
      (bind _output_get (set `self.FallingTime` (+ (`self.FallingTime`) DeltaSeconds)))
      (if (> _output_get (`self.MaxFallingTime`))
        (`self.respawn`)))))

(event `respawn`
  (bind _cube (`self.Cube`))
  (`self.K2_SetActorTransform` (`self.StartTransform`))
  (`PrimitiveComponent.SetPhysicsLinearVelocity` _cube (0.0 0.0 0.0) false "None")
  (`PrimitiveComponent.SetPhysicsAngularVelocityInRadians` _cube (0.0 0.0 0.0) false "None")
  (set `self.FallingTime` 0.0))

(fn `UserConstructionScript`)