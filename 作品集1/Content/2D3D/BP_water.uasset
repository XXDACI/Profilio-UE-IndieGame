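; BP_water is a water hazard that hurts the third-person player character on contact, unless lava has disabled its collision.
; An overlap with a component tagged "lava" switches the water collision off.
; Any other overlap casts the actor to BP_ThirdPersonCharacter and calls Hurt with a fixed damage amount.
; A reset event restores query-only collision, and debug prints mark both overlap branches.
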(event `self.water_collision.OnComponentBeginOverlap`
  (params (OverlappedComponent :type "PrimitiveComponent Object Reference") (OtherActor :type "Actor Object Reference") (OtherComp :type "PrimitiveComponent Object Reference") (OtherBodyIndex :type Integer) (bFromSweep :type Boolean) (SweepResult :type "HitResult Structure (by ref)"))
  (if (`ActorComponent.ComponentHasTag` OtherComp "lava")
    (`KismetSystemLibrary.PrintString` "lava")
    (`PrimitiveComponent.SetCollisionEnabled` (`self.water_collision`) "NoCollision")
    (else
      (`KismetSystemLibrary.PrintString` "false")
      (bind _asbp_third_person_character (cast `/Game/ThirdPerson/Blueprints/BP_ThirdPersonCharacter` OtherActor))
      (`/Game/ThirdPerson/Blueprints/BP_ThirdPersonCharacter.Hurt` _asbp_third_person_character 100.0))))

(event `reset`
  (`PrimitiveComponent.SetCollisionEnabled` (`self.water_collision`) "QueryOnly"))

(fn `UserConstructionScript`)