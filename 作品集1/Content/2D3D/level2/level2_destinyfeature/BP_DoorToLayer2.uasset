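; Door actor in the level 2 destiny feature that teleports the third-person character when it overlaps the box trigger.
; The Out flag sends the player to OutCor; otherwise they go to TPbackCor, and the first such trip sets Layer2 on BP_Tablet and caches it in IsLayer2.
; Hide and appear events toggle cube visibility and trigger collision, while reset clears both flags and resets the tablet.
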(event `self.ReceiveTick`
  (params (DeltaSeconds :type "Float (single-precision)")))

(event `self.Box.OnComponentBeginOverlap`
  (params (OverlappedComponent :type "PrimitiveComponent Object Reference") (OtherActor :type "Actor Object Reference") (OtherComp :type "PrimitiveComponent Object Reference") (OtherBodyIndex :type Integer) (bFromSweep :type Boolean) (SweepResult :type "HitResult Structure (by ref)"))
  (bind _out_ (`self.out?`))
  (`KismetSystemLibrary.PrintString` (`KismetStringLibrary.Conv_BoolToString` _out_))
  (if _out_
    (bind _asbp_third_person_character (cast `/Game/ThirdPerson/Blueprints/BP_ThirdPersonCharacter` OtherActor))
    (`self.K2_SetActorLocation` _asbp_third_person_character (`self.out cor`) false false)
    (elif (`self.isLayer2`)
      (bind _asbp_third_person_character_2 (cast `/Game/ThirdPerson/Blueprints/BP_ThirdPersonCharacter` OtherActor))
      (`self.K2_SetActorLocation` _asbp_third_person_character_2 (`self.TPbackCor`) false false)
      (else
        (bind _asbp_third_person_character_3 (cast `/Game/ThirdPerson/Blueprints/BP_ThirdPersonCharacter` OtherActor))
        (`self.K2_SetActorLocation` _asbp_third_person_character_3 (`self.TPbackCor`) false false)
        (bind _returnvalue (`GameplayStatics.GetActorOfClass` "/Game/2D3D/level1/trape/BP_Tablet.BP_Tablet_C"))
        (bind _output_get (set `/Game/2D3D/level1/trape/BP_Tablet.layer2` true _returnvalue))
        (set `self.isLayer2` _output_get)))))

(event `hide`
  (`SceneComponent.SetHiddenInGame` (`self.Cube`) true false)
  (`PrimitiveComponent.SetCollisionEnabled` (`self.Box`) "NoCollision"))

(event `appear`
  (`SceneComponent.SetHiddenInGame` (`self.Cube`) false false)
  (`PrimitiveComponent.SetCollisionEnabled` (`self.Box`) "QueryOnly"))

(event `reset`
  (set `self.out?` false)
  (set `self.isLayer2` false)
  (bind _returnvalue (`GameplayStatics.GetActorOfClass` "/Game/2D3D/level1/trape/BP_Tablet.BP_Tablet_C"))
  (`/Game/2D3D/level1/trape/BP_Tablet.reset` _returnvalue))

(fn `UserConstructionScript`)