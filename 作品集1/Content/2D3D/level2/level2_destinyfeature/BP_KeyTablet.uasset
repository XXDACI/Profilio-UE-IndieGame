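; Key tablet actor in the level 2 destiny feature that randomly arranges two cubes between a close and a far position.
; BeginPlay caches the relative locations of Cube1 as Close and Cube as Far.
; The randomPlatform event picks one of the two arrangements at random and applies it through locationSet without sweeping.
; Its debug print rolls separately from the branch, so the printed number can differ from the result.
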(event `self.ReceiveBeginPlay`
  (set `self.close` (`SceneComponent.RelativeLocation` (`self.Cube1`)))
  (set `self.far` (`SceneComponent.RelativeLocation` (`self.Cube`))))

(event `randomPlatform`
  (bind _returnvalue (`KismetMathLibrary.RandomInteger` 2))
  (`KismetSystemLibrary.PrintString` (`KismetStringLibrary.Conv_IntToString` _returnvalue))
  (if (== _returnvalue 0)
    (`self.location Set` (`self.close`) (`self.far`))
    (else
      (`self.location Set` (`self.far`) (`self.close`)))))

(event `location Set`
  (params (cube0 :type "Vector Structure") (cube1 :type "Vector Structure"))
  (`SceneComponent.K2_SetRelativeLocation` (`self.Cube`) cube0 false false)
  (`SceneComponent.K2_SetRelativeLocation` (`self.Cube1`) cube1 false false))

(fn `UserConstructionScript`)