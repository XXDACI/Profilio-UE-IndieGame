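; BP_RollingRock is a rock hazard for level 2 that travels a fixed straight path and damages the player it touches.
; It starts hidden with collision off; StartRoll reveals it and a timeline moves it along world X from its start location.
; Sphere overlap calls Hurt on BP_ThirdPersonCharacter, and reset returns the rock to its start, hidden again.
; The setActive flag is inverted: true means hidden and harmless.
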(event `self.ReceiveBeginPlay`
  (set `self.startLocation` (`self.K2_GetActorLocation`))
  (`self.setActive` true))

(event `self.Sphere1.OnComponentBeginOverlap`
  (params (OverlappedComponent :type "PrimitiveComponent Object Reference") (OtherActor :type "Actor Object Reference") (OtherComp :type "PrimitiveComponent Object Reference") (OtherBodyIndex :type Integer) (bFromSweep :type Boolean) (SweepResult :type "HitResult Structure (by ref)"))
  (bind _asbp_third_person_character (cast `/Game/ThirdPerson/Blueprints/BP_ThirdPersonCharacter` OtherActor))
  (`/Game/ThirdPerson/Blueprints/BP_ThirdPersonCharacter.Hurt` _asbp_third_person_character 100.0)
  (`KismetSystemLibrary.PrintString` "hurt"))

(event `reset`
  (`self.setActive` true)
  (`self.K2_SetActorLocation` (`self.startLocation`)))

(event `StartRoll`
  (`self.setActive` false)
  (bind (_direction _alpha) (`Timeline|TL_Roll` :!via `PlayFromStart`)
    (:`Update`
      (`self.K2_SetActorLocation` (`KismetMathLibrary.MakeVector` (+ (* _alpha 10300.0) (.x (`self.startLocation`))) (.y (`self.startLocation`)) (.z (`self.startLocation`)))))))

(event `setActive`
  (params (active :type Boolean))
  (bind _sphere1 (`self.Sphere1`))
  (`self.SetActorHiddenInGame` active)
  (if active
    (`PrimitiveComponent.SetCollisionEnabled` _sphere1 "NoCollision")
    (else
      (`PrimitiveComponent.SetCollisionEnabled` _sphere1 "QueryOnly"))))

(fn `UserConstructionScript`)