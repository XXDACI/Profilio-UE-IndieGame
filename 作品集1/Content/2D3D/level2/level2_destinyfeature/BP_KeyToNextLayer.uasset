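; BP_KeyToNextLayer is a trigger actor that resizes level walls while the third-person player overlaps it.
; Entering its WallControl component adds 2 to the X scale of every BP_Walls actor in the level.
; Leaving subtracts the same amount and destroys the key from inside that wall loop, making it single-use when any walls exist.
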(event `self.wallControl.OnComponentBeginOverlap`
  (params (OverlappedComponent :type "PrimitiveComponent Object Reference") (OtherActor :type "Actor Object Reference") (OtherComp :type "PrimitiveComponent Object Reference") (OtherBodyIndex :type Integer) (bFromSweep :type Boolean) (SweepResult :type "HitResult Structure (by ref)"))
  (cast `/Game/ThirdPerson/Blueprints/BP_ThirdPersonCharacter` OtherActor)
  (bind _outactors (`GameplayStatics.GetAllActorsOfClass` "/Game/2D3D/level2/level2_destinyfeature/BP_Walls.BP_Walls_C"))
  (for _array_element _outactors
    (`self.SetActorScale3D` _array_element (`KismetMathLibrary.MakeVector` (+ (.x (`self.GetActorScale3D` _array_element)) 2.0) (.y (`self.GetActorScale3D` _array_element)) (.z (`self.GetActorScale3D` _array_element))))))

(event `self.wallControl.OnComponentEndOverlap`
  (params (OverlappedComponent :type "PrimitiveComponent Object Reference") (OtherActor :type "Actor Object Reference") (OtherComp :type "PrimitiveComponent Object Reference") (OtherBodyIndex :type Integer))
  (cast `/Game/ThirdPerson/Blueprints/BP_ThirdPersonCharacter` OtherActor)
  (bind _outactors (`GameplayStatics.GetAllActorsOfClass` "/Game/2D3D/level2/level2_destinyfeature/BP_Walls.BP_Walls_C"))
  (for _array_element _outactors
    (`self.SetActorScale3D` _array_element (`KismetMathLibrary.MakeVector` (- (.x (`self.GetActorScale3D` _array_element)) 2.0) (.y (`self.GetActorScale3D` _array_element)) (.z (`self.GetActorScale3D` _array_element))))
    (`self.K2_DestroyActor`)))

(fn `UserConstructionScript`)