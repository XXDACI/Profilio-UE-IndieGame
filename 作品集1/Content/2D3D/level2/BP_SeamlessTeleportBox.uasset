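; Seamless two-door puzzle box that loops the player until they pick the non-fake entrance three times in a row.
; Random DoorNum marks one entrance frame with FakeColor; right picks increment Score, wrong picks reset it.
; Until the third success, entering teleports the player to the matching exit by relative transform, recolors exit frames and rerolls.
; Overlap-driven timelines slide doors, opening exit fronts alongside entrance fronts to mirror the view.
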(event `self.ReceiveBeginPlay`
  (`self.RandomDoorNum`)
  (if (== (`self.doorNum`) 1)
    (`self.Entrance1Fake`)
    (else
      (`self.Entrance2Fake`))))

(event `RandomDoorNum`
  (set `self.doorNum` (`KismetMathLibrary.RandomInteger` 2)))

(event `self.Entrance1.OnComponentBeginOverlap`
  (params (OverlappedComponent :type "PrimitiveComponent Object Reference") (OtherActor :type "Actor Object Reference") (OtherComp :type "PrimitiveComponent Object Reference") (OtherBodyIndex :type Integer) (bFromSweep :type Boolean) (SweepResult :type "HitResult Structure (by ref)"))
  (if (== OtherActor (`GameplayStatics.GetPlayerCharacter` 0))
    (if (== (`self.doorNum`) 0)
      (bind _output_get (set `self.score` (+ (`self.score`) 1)))
      (`KismetSystemLibrary.PrintString` (`KismetStringLibrary.Conv_IntToString` _output_get))
      (if (not (== _output_get 3))
        (`self.exit2Fake`)
        (`self.K2_SetActorTransform` (`GameplayStatics.GetPlayerCharacter` 0) (`self.GetTargetTransform1`) false false :!label _label)
        (`self.RandomDoorNum` :!label _label_2)
        (if (== (`self.doorNum`) 1)
          (`self.Entrance1Fake`)
          (else
            (`self.Entrance2Fake`))))
      (else
        (bind _output_get_2 (set `self.score` 0))
        (`KismetSystemLibrary.PrintString` (`KismetStringLibrary.Conv_IntToString` _output_get_2))
        (`self.exit1Fake`)
        (goto _label)))))

(event `self.Entrance2.OnComponentBeginOverlap`
  (params (OverlappedComponent :type "PrimitiveComponent Object Reference") (OtherActor :type "Actor Object Reference") (OtherComp :type "PrimitiveComponent Object Reference") (OtherBodyIndex :type Integer) (bFromSweep :type Boolean) (SweepResult :type "HitResult Structure (by ref)"))
  (if (== OtherActor (`GameplayStatics.GetPlayerCharacter` 0))
    (if (== (`self.doorNum`) 1)
      (`self.exit1Fake`)
      (bind _output_get (set `self.score` (+ (`self.score`) 1)))
      (`KismetSystemLibrary.PrintString` (`KismetStringLibrary.Conv_IntToString` _output_get))
      (if (not (== _output_get 3))
        (`self.K2_SetActorTransform` (`GameplayStatics.GetPlayerCharacter` 0) (`self.GetTargetTransform2`) false false :!label _label_3)
        (goto _label_2))
      (else
        (`self.exit2Fake`)
        (bind _output_get_2 (set `self.score` 0))
        (`KismetSystemLibrary.PrintString` (`KismetStringLibrary.Conv_IntToString` _output_get_2))
        (goto _label_3)))))

(event `Entrance1Fake`
  ; color change
  (`self.ChangeColor` (`self.en1left`) (`self.en1top`) (`self.en1right`) (`self.en2left`) (`self.en2top`) (`self.en2right`) (`self.fakeColor`) (`self.originColor`)))

(event `Entrance2Fake`
  ; color change
  (`self.ChangeColor` (`self.en2left`) (`self.en2top`) (`self.en2right`) (`self.en1left`) (`self.en1top`) (`self.en1right`) (`self.fakeColor`) (`self.originColor`)))

(event `reset`
  (bind _origincolor (`self.originColor`))
  ; reset
  (set `self.score` 0)
  (`self.ChangeColor` (`self.ex2left`) (`self.ex2top`) (`self.ex2right`) (`self.ex1left`) (`self.ex1top`) (`self.ex1right`) _origincolor _origincolor)
  (`self.RandomDoorNum`)
  (if (== (`self.doorNum`) 1)
    (`self.Entrance1Fake`)
    (else
      (`self.Entrance2Fake`))))

(event `exit1Fake`
  ; color change
  (`self.ChangeColor` (`self.ex1left`) (`self.ex1top`) (`self.ex1right`) (`self.ex2left`) (`self.ex2top`) (`self.ex2right`) (`self.fakeColor`) (`self.originColor`)))

(event `exit2Fake`
  ; color change
  (`self.ChangeColor` (`self.ex2left`) (`self.ex2top`) (`self.ex2right`) (`self.ex1left`) (`self.ex1top`) (`self.ex1right`) (`self.fakeColor`) (`self.originColor`)))

(event `self.ex1frontCol.OnComponentBeginOverlap`
  (params (OverlappedComponent :type "PrimitiveComponent Object Reference") (OtherActor :type "Actor Object Reference") (OtherComp :type "PrimitiveComponent Object Reference") (OtherBodyIndex :type Integer) (bFromSweep :type Boolean) (SweepResult :type "HitResult Structure (by ref)"))
  ; door open/close
  (bind (_direction _tl_lift) (`Timeline|Timeline` :!label _label_4)
    (:`Update`
      (`SceneComponent.K2_SetRelativeLocation` (`self.ex1front`) (`KismetMathLibrary.VLerp` (`self.frontClosepos`) (`self.frontOpenpos`) _tl_lift) false false))))

(event `self.ex1backCol.OnComponentBeginOverlap`
  (params (OverlappedComponent :type "PrimitiveComponent Object Reference") (OtherActor :type "Actor Object Reference") (OtherComp :type "PrimitiveComponent Object Reference") (OtherBodyIndex :type Integer) (bFromSweep :type Boolean) (SweepResult :type "HitResult Structure (by ref)"))
  ; door open/close
  (bind (_direction _tl_lift) (`Timeline|Timeline_3` :!label _label_5)
    (:`Update`
      (`SceneComponent.K2_SetRelativeLocation` (`self.ex1back`) (`KismetMathLibrary.VLerp` (`self.backClosepos`) (`self.backOpenpos`) _tl_lift) false false))))

(event `self.ex1frontCol.OnComponentEndOverlap`
  (params (OverlappedComponent :type "PrimitiveComponent Object Reference") (OtherActor :type "Actor Object Reference") (OtherComp :type "PrimitiveComponent Object Reference") (OtherBodyIndex :type Integer))
  ; door open/close
  (goto _label_4 :!via `Reverse`))

(event `self.ex1backCol.OnComponentEndOverlap`
  (params (OverlappedComponent :type "PrimitiveComponent Object Reference") (OtherActor :type "Actor Object Reference") (OtherComp :type "PrimitiveComponent Object Reference") (OtherBodyIndex :type Integer))
  ; door open/close
  (goto _label_5 :!via `Reverse`))

(event `self.en1frontCol.OnComponentBeginOverlap`
  (params (OverlappedComponent :type "PrimitiveComponent Object Reference") (OtherActor :type "Actor Object Reference") (OtherComp :type "PrimitiveComponent Object Reference") (OtherBodyIndex :type Integer) (bFromSweep :type Boolean) (SweepResult :type "HitResult Structure (by ref)"))
  ; door open/close
  (bind (_direction _tl_lift) (`Timeline|Timeline_0` :!label _label_6)
    (:`Update`
      (bind _returnvalue (`KismetMathLibrary.VLerp` (`self.frontClosepos`) (`self.frontOpenpos`) _tl_lift))
      (`SceneComponent.K2_SetRelativeLocation` (`self.en1front`) _returnvalue false false)
      (`SceneComponent.K2_SetRelativeLocation` (`self.ex1front`) _returnvalue false false))))

(event `self.en1backCol.OnComponentBeginOverlap`
  (params (OverlappedComponent :type "PrimitiveComponent Object Reference") (OtherActor :type "Actor Object Reference") (OtherComp :type "PrimitiveComponent Object Reference") (OtherBodyIndex :type Integer) (bFromSweep :type Boolean) (SweepResult :type "HitResult Structure (by ref)"))
  ; door open/close
  (bind (_direction _tl_lift) (`Timeline|Timeline_4` :!label _label_7)
    (:`Update`
      (`SceneComponent.K2_SetRelativeLocation` (`self.en1back`) (`KismetMathLibrary.VLerp` (`self.backClosepos`) (`self.backOpenpos`) _tl_lift) false false))))

(event `self.en1frontCol.OnComponentEndOverlap`
  (params (OverlappedComponent :type "PrimitiveComponent Object Reference") (OtherActor :type "Actor Object Reference") (OtherComp :type "PrimitiveComponent Object Reference") (OtherBodyIndex :type Integer))
  ; door open/close
  (goto _label_6 :!via `Reverse`))

(event `self.en1backCol.OnComponentEndOverlap`
  (params (OverlappedComponent :type "PrimitiveComponent Object Reference") (OtherActor :type "Actor Object Reference") (OtherComp :type "PrimitiveComponent Object Reference") (OtherBodyIndex :type Integer))
  ; door open/close
  (goto _label_7 :!via `Reverse`))

(event `self.ex2frontCol.OnComponentBeginOverlap`
  (params (OverlappedComponent :type "PrimitiveComponent Object Reference") (OtherActor :type "Actor Object Reference") (OtherComp :type "PrimitiveComponent Object Reference") (OtherBodyIndex :type Integer) (bFromSweep :type Boolean) (SweepResult :type "HitResult Structure (by ref)"))
  ; door open/close
  (bind (_direction _tl_lift) (`Timeline|Timeline_1` :!label _label_8)
    (:`Update`
      (`SceneComponent.K2_SetRelativeLocation` (`self.ex2front`) (`KismetMathLibrary.VLerp` (`self.frontClosepos`) (`self.frontOpenpos`) _tl_lift) false false))))

(event `self.ex2backCol.OnComponentBeginOverlap`
  (params (OverlappedComponent :type "PrimitiveComponent Object Reference") (OtherActor :type "Actor Object Reference") (OtherComp :type "PrimitiveComponent Object Reference") (OtherBodyIndex :type Integer) (bFromSweep :type Boolean) (SweepResult :type "HitResult Structure (by ref)"))
  ; door open/close
  (bind (_direction _tl_lift) (`Timeline|Timeline_5` :!label _label_9)
    (:`Update`
      (`SceneComponent.K2_SetRelativeLocation` (`self.ex2back`) (`KismetMathLibrary.VLerp` (`self.backClosepos`) (`self.backOpenpos`) _tl_lift) false false))))

(event `self.ex2frontCol.OnComponentEndOverlap`
  (params (OverlappedComponent :type "PrimitiveComponent Object Reference") (OtherActor :type "Actor Object Reference") (OtherComp :type "PrimitiveComponent Object Reference") (OtherBodyIndex :type Integer))
  ; door open/close
  (goto _label_8 :!via `Reverse`))

(event `self.ex2backCol.OnComponentEndOverlap`
  (params (OverlappedComponent :type "PrimitiveComponent Object Reference") (OtherActor :type "Actor Object Reference") (OtherComp :type "PrimitiveComponent Object Reference") (OtherBodyIndex :type Integer))
  ; door open/close
  (goto _label_9 :!via `Reverse`))

(event `self.en2frontCol.OnComponentBeginOverlap`
  (params (OverlappedComponent :type "PrimitiveComponent Object Reference") (OtherActor :type "Actor Object Reference") (OtherComp :type "PrimitiveComponent Object Reference") (OtherBodyIndex :type Integer) (bFromSweep :type Boolean) (SweepResult :type "HitResult Structure (by ref)"))
  ; door open/close
  (bind (_direction _tl_lift) (`Timeline|Timeline_2` :!label _label_10)
    (:`Update`
      (bind _returnvalue (`KismetMathLibrary.VLerp` (`self.frontClosepos`) (`self.frontOpenpos`) _tl_lift))
      (`SceneComponent.K2_SetRelativeLocation` (`self.en2front`) _returnvalue false false)
      (`SceneComponent.K2_SetRelativeLocation` (`self.ex2front`) _returnvalue false false))))

(event `self.en2backCol.OnComponentBeginOverlap`
  (params (OverlappedComponent :type "PrimitiveComponent Object Reference") (OtherActor :type "Actor Object Reference") (OtherComp :type "PrimitiveComponent Object Reference") (OtherBodyIndex :type Integer) (bFromSweep :type Boolean) (SweepResult :type "HitResult Structure (by ref)"))
  ; door open/close
  (bind (_direction _tl_lift) (`Timeline|Timeline_6` :!label _label_11)
    (:`Update`
      (`SceneComponent.K2_SetRelativeLocation` (`self.en2back`) (`KismetMathLibrary.VLerp` (`self.backClosepos`) (`self.backOpenpos`) _tl_lift) false false))))

(event `self.en2frontCol.OnComponentEndOverlap`
  (params (OverlappedComponent :type "PrimitiveComponent Object Reference") (OtherActor :type "Actor Object Reference") (OtherComp :type "PrimitiveComponent Object Reference") (OtherBodyIndex :type Integer))
  ; door open/close
  (goto _label_10 :!via `Reverse`))

(event `self.en2backCol.OnComponentEndOverlap`
  (params (OverlappedComponent :type "PrimitiveComponent Object Reference") (OtherActor :type "Actor Object Reference") (OtherComp :type "PrimitiveComponent Object Reference") (OtherBodyIndex :type Integer))
  ; door open/close
  (goto _label_11 :!via `Reverse`))

(fn `ChangeColor`
  (params (left1 :type "PrimitiveComponent Object Reference") (top1 :type "PrimitiveComponent Object Reference") (right1 :type "PrimitiveComponent Object Reference") (left2 :type "PrimitiveComponent Object Reference") (top2 :type "PrimitiveComponent Object Reference") (right2 :type "PrimitiveComponent Object Reference") (material1 :type "Material Object Reference") (material2 :type "Material Object Reference"))
  (`PrimitiveComponent.SetMaterial` left1 0 material1)
  (`PrimitiveComponent.SetMaterial` top1 0 material1)
  (`PrimitiveComponent.SetMaterial` right1 0 material1)
  (`PrimitiveComponent.SetMaterial` left2 0 material2)
  (`PrimitiveComponent.SetMaterial` top2 0 material2)
  (`PrimitiveComponent.SetMaterial` right2 0 material2))

(fn `GetTargetTransform1`
  (returns (ReturnValue :type "Transform Structure"))
  (return (`KismetMathLibrary.ComposeTransforms` (`KismetMathLibrary.MakeRelativeTransform` (`self.GetTransform` (`GameplayStatics.GetPlayerCharacter` 0)) (`SceneComponent.K2_GetComponentToWorld` (`self.Entrance1`))) (`SceneComponent.K2_GetComponentToWorld` (`self.Exit1`)))))

(fn `GetTargetTransform2`
  (returns (ReturnValue :type "Transform Structure"))
  (return (`KismetMathLibrary.ComposeTransforms` (`KismetMathLibrary.MakeRelativeTransform` (`self.GetTransform` (`GameplayStatics.GetPlayerCharacter` 0)) (`SceneComponent.K2_GetComponentToWorld` (`self.Entrance2`))) (`SceneComponent.K2_GetComponentToWorld` (`self.Exit2`)))))

(fn `UserConstructionScript`
  (`BoxComponent.SetBoxExtent` (`self.Entrance1`) (`self.BoxSize`) true)
  (`BoxComponent.SetBoxExtent` (`self.Exit1`) (`self.BoxSize`) true)
  (`BoxComponent.SetBoxExtent` (`self.Entrance2`) (`self.BoxSize`) true)
  (`BoxComponent.SetBoxExtent` (`self.Exit2`) (`self.BoxSize`) true))