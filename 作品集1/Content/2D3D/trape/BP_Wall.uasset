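; BP_Wall is a wall actor in the 2D3D trap folder whose Box1 component can be stretched and restored on demand.
; BeginPlay caches Box1's world scale.
; The setboxnewscale event sets the box's Y scale to a very large fixed value while keeping X and Z, and setboxoldscale reapplies the cached scale.
; Nothing in this Blueprint calls either event.
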(event `self.ReceiveBeginPlay`
  (set `self.old scale` (`SceneComponent.K2_GetComponentScale` (`self.Box1`))))

(event `set box new scale`
  (bind _box1 (`self.Box1`))
  (`SceneComponent.SetWorldScale3D` _box1 (`KismetMathLibrary.MakeVector` (.x (`SceneComponent.K2_GetComponentScale` _box1)) 3000.0 (.z (`SceneComponent.K2_GetComponentScale` _box1)))))

(event `set box old scale`
  (`SceneComponent.SetWorldScale3D` (`self.Box1`) (`self.old scale`)))

(fn `UserConstructionScript`)